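; Track tile for a three-lane runner that fills itself with random obstacles.
; On BeginPlay it picks two of the left, center and right lanes, then spawns at each either nothing or one of four obstacle types (enemy, jump, break, sprint).
; When the ThirdPersonCharacter overlaps its box, it has the ThirdPersonGameMode spawn another tile, then destroys itself after a short delay.
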(event OnComponentBeginOverlap(Box)
  (params (OverlappedComponent :type Primitive%20Component%20Object%20Reference) (OtherActor :type Actor%20Object%20Reference) (OtherComp :type Primitive%20Component%20Object%20Reference) (OtherBodyIndex :type Integer) (bFromSweep :type Boolean) (SweepResult :type Hit%20Result%20Structure%20%28by%20ref%29))
  (Utilities|Casting|CastToThirdPersonCharacter OtherActor)
  (bind _asthird_person_game_mode (Utilities|Casting|CastToThirdPersonGameMode (Game|GetGameMode)))
  (Default|SpawnTile _asthird_person_game_mode)
  (Utilities|FlowControl|Delay 1.0)
  (Actor|DestroyActor))

(event EventBeginPlay
  (CallFunction|ChooseLanetoSpawnObstacles))

(event Collision|EventActorBeginOverlap
  (params (OtherActor :type Actor%20Object%20Reference)))

(event EventTick
  (params (DeltaSeconds :type Float%20%28single-precision%29)))

(fn ConstructionScript)

(fn ChooseLanetoSpawnObstacles
  ;[1 1 1 1 30] Les obstacles peuvent pop sur 2 des 3 lanes
  (switch int (Math|Random|RandomIntegerinRange 0 2)
    (:0
      ;[1 1 1 1 30] Obstacles à Gauche et au Centre
      ;;[1 1 1] Lane Left
      (CallFunction|SpawnObstacles (Transformation|GetWorldTransform (Variables|Default|GetLaneLeft)))
      ;;[1 1 1] Lane Center
      (CallFunction|SpawnObstacles (Transformation|GetWorldTransform (Variables|Default|GetLaneCenter))))
    (:1
      ;[1 1 1 1 30] Obstacles au Centre et à Droite
      ;;[1 1 1] Lane Center
      (CallFunction|SpawnObstacles (Transformation|GetWorldTransform (Variables|Default|GetLaneCenter)))
      ;;[1 1 1] Lane Right
      (CallFunction|SpawnObstacles (Transformation|GetWorldTransform (Variables|Default|GetLaneRight))))
    (:2
      ;[1 1 1 1 30] Obstacles à Gauche et à Droite
      ;;[1 1 1] Lane Left
      (CallFunction|SpawnObstacles (Transformation|GetWorldTransform (Variables|Default|GetLaneLeft)))
      ;;[1 1 1] Lane Right
      (CallFunction|SpawnObstacles (Transformation|GetWorldTransform (Variables|Default|GetLaneRight))))))

(fn SpawnObstacles
  (params (NewParam :type Transform))
  (switch int (Math|Random|RandomIntegerinRange 0 4)
    (:0
      _)
    (:1
      (Game|SpawnActorfromClass "/Game/Run/BP/BP_ObstacleEnemy.BP_ObstacleEnemy_C" NewParam "Undefined" 0 0))
    (:2
      (Game|SpawnActorfromClass "/Game/Run/BP/BP_ObstacleJump.BP_ObstacleJump_C" NewParam "Undefined" 0 0))
    (:3
      (Game|SpawnActorfromClass "/Game/Run/BP/BP_ObstacleBreak.BP_ObstacleBreak_C" NewParam "Undefined" 0 0))
    (:4
      (Game|SpawnActorfromClass "/Game/Run/BP/BP_OBstacleSprint.BP_ObstacleSprint_C" NewParam "Undefined" 0 0)))
  (return))